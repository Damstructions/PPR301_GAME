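; Enemy character Blueprint with a melee attack, damage intake, ragdoll death and adjustable walk speed.
; Attack sphere-traces for pawns at the right-hand socket and applies damage, throttled by a briefly delayed DoOnce.
; AnyDamage lowers Health and binds OnDeath to BPCHealthSystem's event, which enables mesh physics and destroys the actor after a delay.
; Montage playback with its attack-end call is unconnected, so attacks play no animation here.
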(event Custom|Attack
  (bind _mesh (Variables|Character|GetMesh))
  (bind _returnvalue (Transformation|GetSocketLocation _mesh "hand_r"))
  ;[1 1 1] Damage to THAT guy (it's a bit of a mess lmao)
  (if (not (Variables|Default|GetDeath))
    (Utilities|FlowControl|DoOnce false :!label _label
      (:Completed
        (bind _outhit (Collision|SphereTraceForObjects _returnvalue _returnvalue 1.5e+02 (Utilities|Array|MakeArray "ObjectTypeQuery3") false 0 "None"))
        (Game|Damage|ApplyDamage (.HitActor (Collision|BreakHitResult _outhit)) (Variables|Default|GetDamage) 0 0)
        (Utilities|FlowControl|Delay 0.1)
        (goto _label Reset)))))

(event Custom|OnDeath
  ;[1 1 1] Damage to THIS one
  (Physics|SetSimulatePhysics (Variables|Character|GetMesh) true)
  (Variables|Default|SetDeath true)
  (Utilities|FlowControl|Delay 5.0)
  (Actor|DestroyActor))

(event Game|Damage|EventAnyDamage
  (params (Damage :type Float%20%28single-precision%29) (DamageType :type Damage%20Type%20Object%20Reference) (InstigatedBy :type Controller%20Object%20Reference) (DamageCauser :type Actor%20Object%20Reference))
  ;[1 1 1] Damage to THIS one
  (Variables|Default|SetHealth (- (Variables|Default|GetHealth) Damage))
  (EventDispatchers|BindEventtoOnDeath (Variables|Default|GetBPC_HealthSystem) (delegate Custom|OnDeath)))

(fn ConstructionScript)

(fn UpdateWalkSPD
  (params (NewWalkSPD :type Float%20%28double-precision%29))
  (Variables|/Script/Engine.CharacterMovementComponent|SetMaxWalkSpeed (Variables|Character|GetCharacterMovement) NewWalkSPD))