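; Chaser enemy that pursues the player and attacks on reaching them.
; ChasePlayer loops through AIMoveTo, re-calling itself on success or failure.
; On a successful move with an attack ready, it casts to BP_FirstPersonCharacter, calls DealDamage and recharges after an ATKRate delay.
; Its own DealDamage event reduces Health, enabling mesh physics and setting Dead at zero, so the next chase call destroys the actor.
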(event Custom|ChasePlayer
  (if (Variables|Default|GetDead?)
    (Actor|DestroyActor) ; Change this to Death animation, Sound, and Disable Collision
    (else
      (AI|AIMoveTo self "0, 0, 0" (Game|GetPlayerCharacter 0) 5.0 false
        (:OnSuccess
          (if (Variables|Default|GetCanATK)
            (Variables|Default|SetCanATK false)
            (CallFunction|RechargeATK)
            ;[1 1 1] DealDMG phase, cast to BP_Player equivalent
            (CallFunction|ChasePlayer)
            (Utilities|Casting|CastToBP_FirstPersonCharacter (Game|GetPlayerCharacter 0))
            (CallFunction|DealDamage (Variables|Default|GetDamageToDo))
            (else
              (CallFunction|ChasePlayer :!label _label))))
        (:OnFail
          (goto _label))))))

(event Custom|RechargeATK
  ;[1 1 1] Recharge Attacks after Delay, set ATKRate!
  (Utilities|FlowControl|Delay (Variables|Default|GetATKRate))
  (Variables|Default|SetCanATK true))

(event Custom|DealDamage
  (params (Damage :type Float%20%28double-precision%29))
  (bind _output_get (Variables|Default|SetHealth (- (Variables|Default|GetHealth) Damage)))
  (if (<= _output_get 0.0)
    (Physics|SetSimulatePhysics (Variables|Character|GetMesh) true)
    (Variables|Default|SetDead? true)))

(event EventBeginPlay
  (Variables|Default|SetHealth (Variables|Default|GetMaxHealth))
  (Utilities|FlowControl|Delay 0.2)
  (CallFunction|ChasePlayer))

(event Collision|EventActorBeginOverlap
  (params (OtherActor :type Actor%20Object%20Reference)))

(event EventTick
  (params (DeltaSeconds :type Float%20%28single-precision%29)))

(fn ConstructionScript)