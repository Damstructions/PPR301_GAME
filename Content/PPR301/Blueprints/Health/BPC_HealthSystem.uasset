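; BPC_HealthSystem is a component that tracks health for the actor it is attached to.
; On BeginPlay it fills Health to MaxHealth and binds to the owner's OnTakeAnyDamage event.
; Each hit subtracts clamped damage, calls the OnTookDamage dispatcher, prints the new health, and calls OnDeath when health is zero or below.
; The Death graph is empty, so the component itself implements no death behaviour.
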(event Custom|TookDamage
  (params (DamagedActor :type Actor%20Object%20Reference) (Damage :type Float%20%28single-precision%29) (DamageType :type Damage%20Type%20Object%20Reference) (InstigatedBy :type Controller%20Object%20Reference) (DamageCauser :type Actor%20Object%20Reference))
  (Variables|Default|SetHealth (Math|Float|Clamp(Float) (- (Variables|Default|GetHealth) Damage) 0.0 (Variables|Default|GetMaxHealth)))
  (Default|CallOnTookDamage Damage)
  (Development|PrintString (Utilities|String|ToString(Float) (Variables|Default|GetHealth)))
  (if (<= (Variables|Default|GetHealth) 0.0)
    (Default|CallOnDeath)))

(event EventBeginPlay
  (Variables|Default|SetOwner (Components|GetOwner))
  (Variables|Default|SetHealth (Variables|Default|GetMaxHealth))
  (EventDispatchers|BindEventtoOnTakeAnyDamage (Variables|Default|GetOwner) (EventDispatchers|CreateEvent :!event Custom|TookDamage)))

(event EventTick
  (params (DeltaSeconds :type Float%20%28single-precision%29)))

(fn Death)