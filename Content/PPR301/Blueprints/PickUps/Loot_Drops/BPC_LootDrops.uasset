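; Actor component that drops a random loot pickup beneath its owner, tied to the owner's death.
; BeginPlay binds to the owner's BPC_HealthSystem OnDeath, then continues into the same spawn logic the death event uses.
; A downward trace places the pickup with random yaw.
; RandomInteger(2) only yields the two ammo pickups, leaving the Select's HealthPickUp option unreachable.
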(event Custom|OnDeath_Event
  (Variables|Default|SetOwner (Components|GetOwner))
  (bind _outhit (Collision|LineTraceByChannel (Transformation|GetActorLocation (Variables|Default|GetOwner)) (- (Transformation|GetActorLocation (Variables|Default|GetOwner)) "0.000000,0.000000,200.000000") "TraceTypeQuery1" false (Utilities|Array|MakeArray (Game|GetPlayerCharacter 0)) "None"))
  (Game|SpawnActorfromClass (Utilities|Select :Index (Math|Random|RandomInteger 2) :Option%200 "/Game/PPR301/Blueprints/PickUps/AmmoPickUp_01.AmmoPickUp_01_C" :Option%201 "/Game/PPR301/Blueprints/PickUps/AmmoPickUp_02.AmmoPickUp_02_C" :Option%202 "/Game/PPR301/Blueprints/PickUps/HealthPickUp.HealthPickUp_C") (Math|Transform|MakeTransform (.Location (Collision|BreakHitResult _outhit)) (Math|Rotator|MakeRotator 0.0 0.0 (Math|Random|RandomFloatinRange 0.0 3.6e+02))) "AlwaysSpawn" "MultiplyWithRoot" 0 0))

(event EventBeginPlay
  (Utilities|IsValid (Variables|Default|GetOwner)
    (:Is%20Valid
      (EventDispatchers|AssignOnDeath (Actor|GetComponentbyClass (Variables|Default|GetOwner) "/Game/PPR301/Blueprints/Health/BPC_HealthSystem.BPC_HealthSystem_C") (delegate Custom|OnDeath_Event))
      (Variables|Default|SetOwner (Components|GetOwner))
      (bind _outhit (Collision|LineTraceByChannel (Transformation|GetActorLocation (Variables|Default|GetOwner)) (- (Transformation|GetActorLocation (Variables|Default|GetOwner)) "0.000000,0.000000,200.000000") "TraceTypeQuery1" false (Utilities|Array|MakeArray (Game|GetPlayerCharacter 0)) "None"))
      (Game|SpawnActorfromClass (Utilities|Select :Index (Math|Random|RandomInteger 2) :Option%200 "/Game/PPR301/Blueprints/PickUps/AmmoPickUp_01.AmmoPickUp_01_C" :Option%201 "/Game/PPR301/Blueprints/PickUps/AmmoPickUp_02.AmmoPickUp_02_C" :Option%202 "/Game/PPR301/Blueprints/PickUps/HealthPickUp.HealthPickUp_C") (Math|Transform|MakeTransform (.Location (Collision|BreakHitResult _outhit)) (Math|Rotator|MakeRotator 0.0 0.0 (Math|Random|RandomFloatinRange 0.0 3.6e+02))) "AlwaysSpawn" "MultiplyWithRoot" 0 0))))

(event EventTick
  (params (DeltaSeconds :type Float%20%28single-precision%29)))