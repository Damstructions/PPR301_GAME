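; BP_SingleUseContainer is a breakable prop that destroys itself and drops a random pickup when an actor overlaps it.
; Overlap applies damage to itself and binds health component death, but continues straight into the same destroy-and-drop path OnDeath uses.
; A 200-unit downward trace, ignoring the player, places one of two ammo pickups or a health pickup at the hit location with random yaw.
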(event Custom|OnDeath
  (bind _returnvalue (Transformation|GetActorLocation))
  (Development|PrintString "itemDrop")
  (Actor|DestroyActor)
  (bind _outhit (Collision|LineTraceByChannel _returnvalue (- _returnvalue "0.000000,0.000000,200.000000") "TraceTypeQuery1" false (Utilities|Array|MakeArray (Game|GetPlayerCharacter 0)) "None"))
  (Game|SpawnActorfromClass (Utilities|Select :Index (Math|Random|RandomInteger 3) :Option%200 "/Game/PPR301/Blueprints/PickUps/AmmoPickUp_01.AmmoPickUp_01_C" :Option%201 "/Game/PPR301/Blueprints/PickUps/AmmoPickUp_02.AmmoPickUp_02_C" :Option%202 "/Game/PPR301/Blueprints/PickUps/HealthPickUp.HealthPickUp_C") (Math|Transform|MakeTransform (.Location (Collision|BreakHitResult _outhit)) (Math|Rotator|MakeRotator 0.0 0.0 (Math|Random|RandomFloatinRange 0.0 3.6e+02))) "AlwaysSpawn" "MultiplyWithRoot" 0 0))

(event Collision|EventActorBeginOverlap
  (params (OtherActor :type Actor%20Object%20Reference))
  (bind _returnvalue (Transformation|GetActorLocation))
  (Game|Damage|ApplyDamage self 1e+01 0 OtherActor)
  (EventDispatchers|BindEventtoOnDeath (Variables|Default|GetBPC_HealthSystem) (delegate Custom|OnDeath))
  (Development|PrintString "itemDrop")
  (Actor|DestroyActor)
  (bind _outhit (Collision|LineTraceByChannel _returnvalue (- _returnvalue "0.000000,0.000000,200.000000") "TraceTypeQuery1" false (Utilities|Array|MakeArray (Game|GetPlayerCharacter 0)) "None"))
  (Game|SpawnActorfromClass (Utilities|Select :Index (Math|Random|RandomInteger 3) :Option%200 "/Game/PPR301/Blueprints/PickUps/AmmoPickUp_01.AmmoPickUp_01_C" :Option%201 "/Game/PPR301/Blueprints/PickUps/AmmoPickUp_02.AmmoPickUp_02_C" :Option%202 "/Game/PPR301/Blueprints/PickUps/HealthPickUp.HealthPickUp_C") (Math|Transform|MakeTransform (.Location (Collision|BreakHitResult _outhit)) (Math|Rotator|MakeRotator 0.0 0.0 (Math|Random|RandomFloatinRange 0.0 3.6e+02))) "AlwaysSpawn" "MultiplyWithRoot" 0 0))

(fn ConstructionScript)